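; BP_RV100 is a configurable RV100 gun actor assembled entirely in its construction script, with no active event logic.
; Variables toggle visibility of barrel, magazine baseplate, follower or bullets, sights, and a thread protector shown only on threaded barrels.
; The chosen barrel and magazine follow the base skeletal mesh through Master Pose Component.
; A final pass applies the gun material to selected parts and separate front and back materials to tritium and fiber sights.
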(event EventBeginPlay)

(event Collision|EventActorBeginOverlap
  (params (OtherActor :type Actor%20Object%20Reference)))

(event EventTick
  (params (DeltaSeconds :type Float%20%28single-precision%29)))

(fn ConstructionScript
  (Utilities|FlowControl|Sequence
    (:then_0
      (Utilities|FlowControl|Sequence
        (:then_0
          ;[1 1 1] Controls which barrel to show
          (if (Utilities|Enum|Equal(Enum) (Variables|Default|GetBarrelType) "NewEnumerator0")
            (Rendering|SetVisibility (Variables|Default|GetSK_RV100_Barrel_Standard) true false)
            (Utilities|Array|Add (Variables|Default|GetSkeletal%20Components) (Variables|Default|GetSK_RV100_Barrel_Standard))
            (Rendering|SetVisibility (Variables|Default|GetSK_RV100_Barrel_Threaded) false false)
            (Utilities|Array|RemoveItem (Variables|Default|GetSkeletal%20Components) (Variables|Default|GetSK_RV100_Barrel_Threaded))
            (Variables|Booleans|SetThreadedBarrel false)
            (else
              (Rendering|SetVisibility (Variables|Default|GetSK_RV100_Barrel_Threaded) true false)
              (Utilities|Array|Add (Variables|Default|GetSkeletal%20Components) (Variables|Default|GetSK_RV100_Barrel_Threaded))
              (Rendering|SetVisibility (Variables|Default|GetSK_RV100_Barrel_Standard) false false)
              (Utilities|Array|RemoveItem (Variables|Default|GetSkeletal%20Components) (Variables|Default|GetSK_RV100_Barrel_Standard))
              (Variables|Booleans|SetThreadedBarrel true))))
        (:then_1
          ;[1 1 1] Controls which magazine baseplate to show
          (if (Utilities|Enum|Equal(Enum) (Variables|Default|GetBaseplateType) "NewEnumerator0")
            (Rendering|SetVisibility (Variables|Default|GetSM_Magazine_Baseplate_Standard) true false)
            (Rendering|SetVisibility (Variables|Default|GetSM_Magazine_Baseplate_Extended) false false)
            (else
              (Rendering|SetVisibility (Variables|Default|GetSM_Magazine_Baseplate_Extended) true false)
              (Rendering|SetVisibility (Variables|Default|GetSM_Magazine_Baseplate_Standard) false false))))
        (:then_2
          ;[1 1 1] Controls whether to show magazine follower or bullets
          (if (Variables|Default|GetMagazine%20is%20Empty)
            (Rendering|SetVisibility (Variables|Default|GetSM_Magazine_Follower) true false)
            (Rendering|SetVisibility (Variables|Default|GetSM_Bullets) false false)
            (else
              (Rendering|SetVisibility (Variables|Default|GetSM_Bullets) true false)
              (Rendering|SetVisibility (Variables|Default|GetSM_Magazine_Follower) false false))))
        (:then_3
          ;[1 1 1] Controls whether to show Thread Protector or not
          (if (and (Variables|Booleans|GetThreadedBarrel) (Variables|Default|GetAdd%20Thread%20Protector))
            (Rendering|SetVisibility (Variables|Default|GetSM_Thread_Protector) true false)
            (else
              (Rendering|SetVisibility (Variables|Default|GetSM_Thread_Protector) false false))))
        (:then_4
          ;[1 1 1] Controls which sights type to show
          (switch Utilities|FlowControl|Switch|SwitchonSights (Variables|Default|GetSights)
            (:NewEnumerator0
              (Rendering|SetVisibility (Variables|Default|GetSM_Sights_Standard) true false)
              (Rendering|SetVisibility (Variables|Default|GetSM_Sights_Tritium) false false)
              (Rendering|SetVisibility (Variables|Default|GetSM_Sights_Fiber) false true))
            (:NewEnumerator1
              (Rendering|SetVisibility (Variables|Default|GetSM_Sights_Tritium) true false)
              (Rendering|SetVisibility (Variables|Default|GetSM_Sights_Standard) false false)
              (Rendering|SetVisibility (Variables|Default|GetSM_Sights_Fiber) false true))
            (:NewEnumerator2
              (Rendering|SetVisibility (Variables|Default|GetSM_Sights_Fiber) true true)
              (Rendering|SetVisibility (Variables|Default|GetSM_Sights_Standard) false false)
              (Rendering|SetVisibility (Variables|Default|GetSM_Sights_Tritium) false false))))
        (:then_5
          ;[1 1 1] Adds all choosed skeletal components to Master Pose Component which is "SK_RV100_Base"
          (Utilities|Array|Add (Variables|Default|GetSkeletal%20Components) (Variables|Default|GetSK_RV100_Magazine))
          (for _array_element (Variables|Default|GetSkeletal%20Components)
            (Class|SkinnedMeshComponent|SetMasterPoseComponent _array_element (Variables|Default|GetSK_RV100_Base) false)))))
    (:then_1
      (Utilities|FlowControl|Sequence
        (:then_0
          ;[1 1 1] Main gun material and all of it's elements
          (Rendering|Material|SetMaterial (Variables|Default|GetSK_RV100_Base) 0 (Variables|Materials|GetGun%20Material)))
        (:then_1
          ;[1 1 1] Tritium colors
          (Rendering|Material|SetMaterial (Variables|Default|GetSM_Sights_Tritium) 1 (Variables|Materials|GetTritium%20Back%20Material))
          (Rendering|Material|SetMaterial (Variables|Default|GetSM_Sights_Tritium) 2 (Variables|Materials|GetTritium%20Front%20Material)))
        (:then_2
          ;[1 1 1] Fiber sticks color
          (Rendering|Material|SetMaterial (Variables|Default|GetSM_Fiber_Sticks) 0 (Variables|Materials|GetFiber%20Back%20Material))
          (Rendering|Material|SetMaterial (Variables|Default|GetSM_Fiber_Sticks) 1 (Variables|Materials|GetFiber%20Front%20Material)))))))